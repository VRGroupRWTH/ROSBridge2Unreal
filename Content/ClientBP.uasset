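; ClientBP is an example ROS client that exercises topic and service communication in both directions from Unreal.
; On BeginPlay it subscribes to a chatter topic, prepares an outgoing topic, and sets up external and self-advertised add-two-ints services.
; Every Tick increments a counter, publishes it as a test string and calls the external service with it.
; Event handlers print received messages and sums, and answer incoming requests by adding both integers.
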(event OnResponse(ExternalService)
  (params (Message :type ROS%20Service%20Base%20Object%20Reference))
  ;[1 1 1] Services
  (bind _asrossrv_add_two_ints (Utilities|Casting|CastToROSSrvAddTwoInts Message))
  (Development|PrintString (Utilities|String|Append "Sum of two Ints: " (Utilities|String|ToString(Integer) (Class|ROSSrvAddTwoInts|SumasInt _asrossrv_add_two_ints)))))

(event OnNewMessage(ReceiveTopic)
  (params (Message :type ROS%20Message%20Base%20Object%20Reference))
  ;[1 1 1] Topics
  (bind _asrosmsg_string (Utilities|Casting|CastToROSMsgString Message))
  (Development|PrintString (Utilities|String|Append "Received: " (Variables|/Script/Rosbridge2Unreal.ROSMsgString|GetData _asrosmsg_string))))

(event OnRequest(OfferedService)
  (params (RequestResponse :type ROS%20Service%20Base%20Object%20Reference))
  ;[1 1 1] Services
  (bind _asrossrv_add_two_ints (Utilities|Casting|CastToROSSrvAddTwoInts RequestResponse))
  (Variables|/Script/Rosbridge2Unreal.ROSSrvAddTwoInts|SetSum _asrossrv_add_two_ints (+ (Variables|/Script/Rosbridge2Unreal.ROSSrvAddTwoInts|GetA _asrossrv_add_two_ints) (Variables|/Script/Rosbridge2Unreal.ROSSrvAddTwoInts|GetB _asrossrv_add_two_ints))))

(event EventBeginPlay
  (bind _receivetopic (Variables|Default|GetReceiveTopic))
  (bind _offeredservice (Variables|Default|GetOfferedService))
  (Utilities|FlowControl|Sequence
    (:then_0
      ;[1 1 1] Topics
      (Utilities|FlowControl|Sequence
        (:then_0
          (Class|ROSTopicHandle|Initialize _receivetopic "/chatter" "/Script/Rosbridge2Unreal.ROSMsgString")
          (Class|ROSTopicHandle|Subscribe _receivetopic))
        (:then_1
          (Class|ROSTopicHandle|Initialize (Variables|Default|GetSendTopic) "/chatter_unreal" "/Script/Rosbridge2Unreal.ROSMsgString"))))
    (:then_1
      ;[1 1 1] Services
      (Class|ROSServiceHandle|Initialize (Variables|Default|GetExternalService) "/add_two_ints" "/Script/Rosbridge2Unreal.ROSSrvAddTwoInts")
      (Class|ROSServiceHandle|Initialize _offeredservice "/add_two_ints_unreal" "/Script/Rosbridge2Unreal.ROSSrvAddTwoInts")
      (Class|ROSServiceHandle|Advertise _offeredservice))))

(event EventTick
  (params (DeltaSeconds :type Float%20%28single-precision%29))
  (Variables|Default|SetCount (+ (Variables|Default|GetCount) 1))
  (Utilities|FlowControl|Sequence
    (:then_0
      ;[1 1 1] Topic
      (Class|ROSTopicHandle|Publish (Variables|Default|GetSendTopic) (Class|ROSMsgString|Create (Utilities|String|Append "Test" (Utilities|String|ToString(Integer) (Variables|Default|GetCount))))))
    (:then_1
      ;[1 1 1] Service
      (Class|ROSServiceHandle|Call (Variables|Default|GetExternalService) (Class|ROSSrvAddTwoInts|CreateRequest (Class|KismetMathLibrary|ToInt64(Integer) (Variables|Default|GetCount)) (Class|KismetMathLibrary|ToInt64(Integer) (* (Variables|Default|GetCount) 2)))))))

(fn ConstructionScript)